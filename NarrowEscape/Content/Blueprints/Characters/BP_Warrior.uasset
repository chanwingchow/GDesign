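; BP_Warrior is a player-controlled 2D sprite warrior with move, jump, dash and attack via Enhanced Input.
; Attacks, dash attacks and dashes play animation overrides, clearing their state flags when completed or cancelled.
; Standing still gives a normal attack, which moving or jumping cancels; attacking while dashing or airborne gives a downward dash attack, which locks out both.
; The sprite yaws to face horizontal input.
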(event `self.ReceivePossessed`
  (params (NewController :type "Controller Object Reference"))
  (bind _asbp_player_controller (cast `/Game/Blueprints/BP_PlayerController` NewController))
  (`EnhancedInputSubsystemInterface.AddMappingContext` (pcsubsystem `EnhancedInputLocalPlayerSubsystem` _asbp_player_controller) "/Game/Input/IMC_Player.IMC_Player" 0 (struct)))

(event `EnhancedInput|/Game/Input/Actions/IA_Attack`
  (params (ActionValue :type Boolean) (ElapsedSeconds :type "Float (double-precision)") (TriggeredSeconds :type "Float (double-precision)") (InputAction :type "InputAction Object Reference" :default "/Game/Input/Actions/IA_Attack.IA_Attack"))
  (bind _returnvalue (`self.GetAnimInstance`))
  (bind _returnvalue_2 (`self.GetVelocity`))
  ; 攻击
  (:`Started`
    (if (or (`self.IsAttacking`) (`self.IsDashAttacking`))
      _
      (elif (or (`self.IsDashing`) (!= (.z _returnvalue_2) 0.0))
        (set `self.IsDashAttacking` true) ; 突进攻击
        (`self.StopJumping`)
        (`self.LaunchCharacter` (0.0 0.0 -80.0) false true)
        (`PaperZDPlaySlotOverrideAction.PlayAnimationOverrideWithCallbacks` _returnvalue (`self.DashAttackAnimSequence`)
          (:`OnCompleted`
            _)
          (:`OnCancelled`
            _))
        (set `self.IsDashAttacking` false)
        (elif (== (`KismetMathLibrary.VSize` _returnvalue_2) 0.0)
          (set `self.IsAttacking` true) ; 攻击
          (`PaperZDPlaySlotOverrideAction.PlayAnimationOverrideWithCallbacks` _returnvalue (`self.AttackAnimSequence`)
            (:`OnCompleted`
              _)
            (:`OnCancelled`
              _))
          (set `self.IsAttacking` false))))))

(event `EnhancedInput|/Game/Input/Actions/IA_Dash`
  (params (ActionValue :type Boolean) (ElapsedSeconds :type "Float (double-precision)") (TriggeredSeconds :type "Float (double-precision)") (InputAction :type "InputAction Object Reference" :default "/Game/Input/Actions/IA_Dash.IA_Dash"))
  (bind _returnvalue (`self.GetVelocity`))
  ; 突进
  (:`Started`
    (if (not (or (`self.IsAttacking`) (`self.IsDashAttacking`) (`self.IsDashing`) (== (`KismetMathLibrary.VSize2D` (`KismetMathLibrary.Conv_VectorToVector2D` _returnvalue)) 0.0)))
      (set `self.IsDashing` true)
      (`self.LaunchCharacter` (`KismetMathLibrary.MakeVector` (.x _returnvalue) (.y _returnvalue) (`KismetMathLibrary.SelectFloat` 200.0 0.0 (== (.z _returnvalue) 0.0))) false true)
      (`PaperZDPlaySlotOverrideAction.PlayAnimationOverrideWithCallbacks` (`self.GetAnimInstance`) (`self.DashAnimSequence`)
        (:`OnCompleted`
          _)
        (:`OnCancelled`
          _))
      (set `self.IsDashing` false))))

(event `EnhancedInput|/Game/Input/Actions/IA_Jump`
  (params (ActionValue :type Boolean) (ElapsedSeconds :type "Float (double-precision)") (TriggeredSeconds :type "Float (double-precision)") (InputAction :type "InputAction Object Reference" :default "/Game/Input/Actions/IA_Jump.IA_Jump"))
  ; 跳跃
  (:`Started`
    (bind _noheavyattack (`self.RemoveLightAttacks`))
    (if (and _noheavyattack (== (.z (`self.GetVelocity`)) 0.0))
      (`GameplayStatics.SpawnSound2D` "/Game/Assets/SoundEffects/NA_Character_Footsteps/Jump/Dirt/DIRT_Pre_Jump_5.DIRT_Pre_Jump_5" 1.0 1.0 0.0 null)
      (`self.Jump`))))

(event `EnhancedInput|/Game/Input/Actions/IA_Move`
  (params (ActionValue :type "Vector2D Structure") (ElapsedSeconds :type "Float (double-precision)") (TriggeredSeconds :type "Float (double-precision)") (InputAction :type "InputAction Object Reference" :default "/Game/Input/Actions/IA_Move.IA_Move"))
  ; 移动
  (:`Triggered`
    (bind _noheavyattack (`self.RemoveLightAttacks`))
    (if _noheavyattack
      (if (not (== ActionValue_X 0.0))
        ;; 根据X轴方向确定角色相对旋转
        (`SceneComponent.K2_SetRelativeRotation` (`self.Sprite`) (`KismetMathLibrary.MakeRotator` 0.0 0.0 (`KismetMathLibrary.SelectFloat` 0.0 180.0 (> ActionValue_X 0.0))) false false))
      (`self.AddMovementInput` (`KismetMathLibrary.MakeVector` ActionValue_X ActionValue_Y)))))

(fn `RemoveLightAttacks`
  (returns (NoHeavyAttack :type Boolean))
  (bind _returnvalue (not (`self.IsDashAttacking`)))
  (if _returnvalue
    (if (`self.IsAttacking`)
      (`PaperZDAnimInstance.StopAllAnimationOverrides` (`self.GetAnimInstance`))
      (set `self.IsAttacking` false)))
  (return _returnvalue))

(fn `UserConstructionScript`)