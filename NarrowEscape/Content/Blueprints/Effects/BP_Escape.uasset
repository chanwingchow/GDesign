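; BP_Escape is an exit point that ends the level when the player character reaches it.
; On BeginPlay it moves itself to a random reachable navigation point within a large radius of its capsule, so its location varies between runs.
; When a BP_Character overlaps the capsule, it copies the character's Points into BP_GameInstance's GotPoints, carrying the score across the level change, then opens the End level.
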(event `self.ReceiveBeginPlay`
  (`self.K2_SetActorLocation` (`NavigationSystemV1.K2_GetRandomReachablePointInRadius` (`SceneComponent.K2_GetComponentLocation` (`self.CapsuleComponent`)) 100000.0 null null)))

(event `self.CapsuleComponent.OnComponentBeginOverlap`
  (params (OverlappedComponent :type "PrimitiveComponent Object Reference") (OtherActor :type "Actor Object Reference") (OtherComp :type "PrimitiveComponent Object Reference") (OtherBodyIndex :type Integer) (bFromSweep :type Boolean) (SweepResult :type "HitResult Structure (by ref)"))
  (bind _asbp_character (cast `/Game/Blueprints/Creatures/BP_Character` OtherActor))
  (bind _asbp_game_instance (cast `/Game/Blueprints/BP_GameInstance` (`GameplayStatics.GetGameInstance`)))
  (set `/Game/Blueprints/BP_GameInstance.GotPoints` (`/Game/Blueprints/Creatures/BP_Creature.Points` _asbp_character) _asbp_game_instance)
  (`GameplayStatics.OpenLevelBySoftObjectPtr` "/Game/Maps/End.End"))

(fn `UserConstructionScript`)