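; Blueprint function library of helpers for making authenticated HTTP requests to the game's backend through the VaRest plugin.
; Request builds a VaRest request with a given verb and content type, adding an Authorization Bearer header from the GameInstance token.
; ProcessURL sends a request to the GameInstance root URL plus a route, then binds the caller's event to its completion.
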(fn `ProcessURL`
  (params (`目标` :type "VaRestRequestJSON Object Reference") (Route :type String) (`事件` :type "Delegate (by ref)"))
  (bind _asbp_game_instance (cast `/Game/Blueprints/BP_GameInstance` (`GameplayStatics.GetGameInstance` null)))
  (`VaRestRequestJSON.ProcessURL` `目标` (`KismetStringLibrary.Concat_StrStr` (`/Game/Blueprints/BP_GameInstance.RootURL` _asbp_game_instance) Route))
  (add `VaRestRequestJSON.OnRequestComplete` `目标` `事件`))

(fn `Request`
  (params (Verb :type "EVaRestRequestVerb Enum" :default "GET") (ContentType :type "EVaRestRequestContentType Enum" :default "x_www_form_urlencoded_url"))
  (returns (ReturnValue :type "VaRestRequestJSON Object Reference"))
  (bind _asbp_game_instance (cast `/Game/Blueprints/BP_GameInstance` (`GameplayStatics.GetGameInstance` null)))
  (bind _returnvalue (`VaRestSubsystem.ConstructVaRestRequestExt` (subsystem `VaRestSubsystem`) Verb ContentType))
  (`VaRestRequestJSON.SetHeader` _returnvalue "Authorization" (`KismetStringLibrary.Concat_StrStr` "Bearer " (`/Game/Blueprints/BP_GameInstance.Token` _asbp_game_instance)))
  (return _returnvalue))