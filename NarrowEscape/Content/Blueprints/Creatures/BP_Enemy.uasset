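; BP_Enemy is a sprite-based enemy creature that chases and attacks the player character when it sees it.
; PawnSensing filters for BP_Character, then attacks if GetForwardAttackable finds a target within attack length, otherwise chases.
; Chasing turns by X direction and uses AI MoveTo toward a point offset from the target along the sprite's forward vector.
; State flags gate both actions, and attacks play an override animation followed by a cooldown.
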(event `self.PawnSensing.OnSeePawn`
  (params (Pawn :type "Pawn Object Reference"))
  ; 在看见角色时，跟随或攻击角色
  (if (not (or (not (`GameplayStatics.ObjectIsA` Pawn "/Game/Blueprints/Creatures/BP_Character.BP_Character_C")) (`self.IsDead`) (`self.IsAttacking`) (`self.IsHurting`)))
    (bind (_outhit _returnvalue) (`self.GetForwardAttackable` (`self.AttackLength`)))
    (if _returnvalue
      (`self.Attack`)
      (else
        (`self.ChaseCharacter` Pawn)))))

(event `Attack`
  ; 攻击角色
  (if (not (or (`self.IsDead`) (`self.IsHurting`) (`self.IsAttacking`) (`self.IsMoving`) (not (`self.CanAttack`))))
    (set `self.CanAttack` false)
    (set `self.IsAttacking` true)
    (`PaperZDPlaySlotOverrideAction.PlayAnimationOverrideWithCallbacks` (`self.AnimInstance`) (`self.AttackAnimSequence`)
      (:`OnCompleted`
        _)
      (:`OnCancelled`
        _))
    (set `self.IsAttacking` false)
    (`KismetSystemLibrary.Delay` 2.0)
    (set `self.CanAttack` true)))

(event `ChaseCharacter`
  (params (Target :type "Actor Object Reference"))
  ; 跟随角色
  (if (not (or (`self.IsDead`) (`self.IsHurting`) (`self.IsAttacking`)))
    (set `self.IsMoving` true)
    (bind (_returnvalue_x _returnvalue) (`self.GetXDestination` Target))
    (`self.Rotate` _returnvalue_x)
    (`|AIMoveTo` self _returnvalue null
      (:`OnSuccess`
        (set `self.IsMoving` false)))))

(fn `AIMoveTo`)

(fn `GetXDestination`
  (params (Target :type "Actor Object Reference"))
  (returns (ReturnValue_X :type "Float (double-precision)") (ReturnValue :type "Vector Structure"))
  (locals (NewLocalVar :type "Vector Structure" :default (0.0 0.0 0.0)))
  ; 返回到目标方向的X和目标位置
  (bind _output_get (set `local.NewLocalVar` (`self.K2_GetActorLocation` Target)))
  (bind _returnvalue_x (`KismetMathLibrary.BreakVector` (- _output_get (`self.K2_GetActorLocation`) (0.0 0.0 0.0))))
  (return _returnvalue_x (- _output_get (* (`SceneComponent.GetForwardVector` (`self.Sprite`)) (`self.AttackOffset`)))))

(fn `UserConstructionScript`
  (`parent.UserConstructionScript`))