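; BP_Creature is a 2D sprite creature with health, melee attacking and facing, animated through animation-instance overrides.
; AnyDamage subtracts clamped HP, then either plays a hurt override that clears IsHurting when finished or cancelled, or plays death once and destroys the actor.
; Rotate flips the sprite's yaw by X direction, steering the forward sphere trace that Damage uses to apply damage to the hit actor.
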(event `self.ReceiveAnyDamage`
  (params (Damage :type "Float (single-precision)") (DamageType :type "DamageType Object Reference") (InstigatedBy :type "Controller Object Reference") (DamageCauser :type "Actor Object Reference"))
  (set `self.IsHurting` true)
  (bind _output_get (set `self.HP` (`KismetMathLibrary.FClamp` (- (`self.HP`) Damage) 0.0 (`self.MaxHP`))))
  (bind _output_get_2 (set `self.IsDead` (== _output_get 0.0)))
  (if _output_get_2
    ; 死亡
    (`/Engine/EditorBlueprintResources/StandardMacros.DoOnce` false
      (:`Completed`
        (`PaperZDPlaySlotOverrideAction.PlayAnimationOverrideWithCallbacks` (`self.AnimInstance`) (`self.DeathAnimSequence`)
          (:`OnCompleted`
            (`KismetSystemLibrary.DelayUntilNextTick`)
            (`self.K2_DestroyActor`)))))
    (else
      ; 受伤
      (`PaperZDPlaySlotOverrideAction.PlayAnimationOverrideWithCallbacks` (`self.AnimInstance`) (`self.HurtAnimSequence`)
        (:`OnCompleted`
          _)
        (:`OnCancelled`
          _))
      (set `self.IsHurting` false))))

(fn `_Damage`
  (params (AttackLength :type "Float (double-precision)") (AttackValue :type "Float (double-precision)"))
  (returns (HitActor :type "Actor Object Reference"))
  ; 对可攻击Actor造成伤害
  (bind (_outhit _returnvalue) (`self.GetForwardAttackable` AttackLength))
  (if _returnvalue
    (bind (_bblockinghit _binitialoverlap _time _distance _location _impactpoint _normal _impactnormal _physmat _hitactor) (`GameplayStatics.BreakHitResult` _outhit))
    (`GameplayStatics.ApplyDamage` _hitactor AttackValue)
    (return _hitactor)))

(fn `Damage`
  (`self._Damage` (`self.AttackLength`) (`self.AttackValue`)))

(fn `GetForwardAttackable`
  (params (Length :type "Float (double-precision)"))
  (returns (OutHit :type "HitResult Structure") (ReturnValue :type Boolean))
  (locals (Forward :type "Vector Structure" :default (0.0 0.0 0.0)))
  (bind _returnvalue (+ (* (`local.Forward`) (`self.AttackOffset`)) (`self.K2_GetActorLocation`)))
  ; 按通道进行球体追踪前方可攻击Pawn
  (bind _output_get (set `local.Forward` (`SceneComponent.GetForwardVector` (`self.Sprite`))))
  (bind (_outhit _returnvalue_2) (`KismetSystemLibrary.SphereTraceSingle` :`Start` _returnvalue :`End` (+ _returnvalue (* _output_get Length)) :`Radius` 30.0 :`TraceChannel` (`self.AttackTraceChannel`) :`DrawDebugType` "ForDuration"))
  (return _outhit _returnvalue_2))

(fn `Rotate`
  (params (X :type "Float (double-precision)"))
  ; 根据X轴方向确定转向
  (if (not (== X 0.0))
    (`SceneComponent.K2_SetRelativeRotation` (`self.Sprite`) (`KismetMathLibrary.MakeRotator` 0.0 0.0 (`KismetMathLibrary.SelectFloat` 0.0 180.0 (> X 0.0))) false false)))

(fn `UserConstructionScript`)