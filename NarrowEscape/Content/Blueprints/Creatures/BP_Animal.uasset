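; BP_Animal is a creature that flees from characters it sees.
; When PawnSensing spots a pawn, it sets IsMoving, passes the X component of the away vector to Rotate, and starts an AI MoveTo.
; GetXDestination mirrors the seen pawn's position through the animal, so the flee distance equals the current separation.
; IsMoving clears only when the move succeeds.
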(event `self.PawnSensing.OnSeePawn`
  (params (Pawn :type "Pawn Object Reference"))
  ; 在看见角色时，远离角色
  (set `self.IsMoving` true)
  (bind (_x _destination) (`self.GetXDestination` Pawn))
  (`self.Rotate` _x)
  (`|AIMoveTo` self _destination null
    (:`OnSuccess`
      (set `self.IsMoving` false))))

(fn `GetXDestination`
  (params (`目标` :type "Actor Object Reference"))
  (returns (X :type "Float (double-precision)") (Destination :type "Vector Structure"))
  (locals (Vector :type "Vector Structure") (Location :type "Vector Structure"))
  ; 返回到目标方向的X和目标位置
  (bind _output_get (set `local.Location` (`self.K2_GetActorLocation`)))
  (bind _returnvalue (- _output_get (`self.K2_GetActorLocation` `目标`)))
  (bind _output_get_2 (set `local.Vector` _returnvalue))
  (return (.x _output_get_2) (+ _output_get _returnvalue)))

(fn `UserConstructionScript`
  (`parent.UserConstructionScript`))