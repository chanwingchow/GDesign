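; Player-controlled creature character with movement, jump, dash, light attack and heavy attack, registering its Enhanced Input context when possessed.
; State booleans gate each action, and animation overrides clear attack and dash states on completion or cancel.
; Attacking while dashing, jumping or falling becomes a downward heavy attack, while moving or jumping cancels light attacks.
; HeavyAttack launches hit creatures forward and up with boosted damage; its trigger is outside these graphs.
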(event `self.ReceiveTick`
  (params (DeltaSeconds :type "Float (single-precision)"))
  (bind (_returnvalue_x _returnvalue_y _returnvalue_z) (`KismetMathLibrary.BreakVector` (`self.GetVelocity`)))
  (`parent.ReceiveTick` DeltaSeconds)
  (set `self.IsFalling` (< _returnvalue_z 0.0))
  (if (and (`self.IsJumping`) (== _returnvalue_z 0.0))
    (set `self.IsJumping` false)))

(event `self.ReceivePossessed`
  (params (NewController :type "Controller Object Reference"))
  (bind _asbp_player_controller (cast `/Game/Blueprints/GameModes/BP_PlayerController` NewController))
  (`EnhancedInputSubsystemInterface.AddMappingContext` (pcsubsystem `EnhancedInputLocalPlayerSubsystem` _asbp_player_controller) "/Game/Input/IMC_Player.IMC_Player" 0 (struct)))

(event `EnhancedInput|/Game/Input/Actions/IA_Attack`
  (params (ActionValue :type Boolean) (ElapsedSeconds :type "Float (double-precision)") (TriggeredSeconds :type "Float (double-precision)") (InputAction :type "InputAction Object Reference" :default "/Game/Input/Actions/IA_Attack.IA_Attack"))
  (bind _animinstance (`self.AnimInstance`))
  ; 攻击
  (:`Started`
    (if (or (`self.IsDead`) (`self.IsHurting`) (`self.IsAttacking`) (`self.IsHeavyAttacking`))
      _
      (elif (or (`self.IsDashing`) (`self.IsJumping`) (`self.IsFalling`))
        (set `self.IsHeavyAttacking` true) ; 重击
        (`self.StopJumping`)
        (`self.LaunchCharacter` (0.0 0.0 -80.0) false true)
        (`PaperZDPlaySlotOverrideAction.PlayAnimationOverrideWithCallbacks` _animinstance (`self.HeavyAttackAnimSequence`)
          (:`OnCompleted`
            _)
          (:`OnCancelled`
            _))
        (set `self.IsHeavyAttacking` false)
        (elif (not (`self.IsMoving`))
          (set `self.IsAttacking` true) ; 攻击
          (`PaperZDPlaySlotOverrideAction.PlayAnimationOverrideWithCallbacks` _animinstance (`self.AttackAnimSequenece`)
            (:`OnCompleted`
              _)
            (:`OnCancelled`
              _))
          (set `self.IsAttacking` false))))))

(event `EnhancedInput|/Game/Input/Actions/IA_Dash`
  (params (ActionValue :type Boolean) (ElapsedSeconds :type "Float (double-precision)") (TriggeredSeconds :type "Float (double-precision)") (InputAction :type "InputAction Object Reference" :default "/Game/Input/Actions/IA_Dash.IA_Dash"))
  (bind (_returnvalue_x _returnvalue_y _returnvalue_z) (`KismetMathLibrary.BreakVector` (`self.GetVelocity`)))
  (bind (_returnvalue_x_2 _returnvalue_y_2) (`KismetMathLibrary.BreakVector2D` (* (`KismetMathLibrary.Normal2D` (`KismetMathLibrary.MakeVector2D` _returnvalue_x _returnvalue_y)) 700.0)))
  ; 突进
  (:`Started`
    (if (not (or (`self.IsDead`) (`self.IsHurting`) (`self.IsHeavyAttacking`) (`self.IsDashing`) (not (`self.IsMoving`))))
      (set `self.IsDashing` true)
      (`self.LaunchCharacter` (`KismetMathLibrary.MakeVector` _returnvalue_x_2 _returnvalue_y_2 (`KismetMathLibrary.SelectFloat` 140.0 0.0 (== _returnvalue_z 0.0))) false true)
      (`PaperZDPlaySlotOverrideAction.PlayAnimationOverrideWithCallbacks` (`self.AnimInstance`) (`self.DashAnimSequence`)
        (:`OnCompleted`
          _)
        (:`OnCancelled`
          _))
      (set `self.IsDashing` false))))

(event `EnhancedInput|/Game/Input/Actions/IA_Jump`
  (params (ActionValue :type Boolean) (ElapsedSeconds :type "Float (double-precision)") (TriggeredSeconds :type "Float (double-precision)") (InputAction :type "InputAction Object Reference" :default "/Game/Input/Actions/IA_Jump.IA_Jump"))
  ; 跳跃
  (:`Started`
    (if (not (or (`self.IsDead`) (`self.IsHurting`) (`self.IsJumping`) (`self.IsHeavyAttacking`)))
      (`self.RemoveLightAttack`)
      (`GameplayStatics.SpawnSound2D` "/Game/Assets/SoundEffects/NA_Character_Footsteps/Jump/Dirt/DIRT_Pre_Jump_5.DIRT_Pre_Jump_5" 1.0 1.0 0.0 null)
      (`self.Jump`)
      (set `self.IsJumping` true))))

(event `EnhancedInput|/Game/Input/Actions/IA_Move`
  (params (ActionValue :type "Vector2D Structure") (ElapsedSeconds :type "Float (double-precision)") (TriggeredSeconds :type "Float (double-precision)") (InputAction :type "InputAction Object Reference" :default "/Game/Input/Actions/IA_Move.IA_Move"))
  ; 移动
  (:`Triggered`
    (if (not (or (`self.IsDead`) (`self.IsHurting`) (`self.IsHeavyAttacking`)))
      (`self.RemoveLightAttack`)
      (set `self.IsMoving` true)
      (`self.Rotate` ActionValue_X)
      (`self.AddMovementInput` (`KismetMathLibrary.MakeVector` ActionValue_X ActionValue_Y))))
  (:`Completed`
    (set `self.IsMoving` false)))

(event `RemoveLightAttack`
  ; 移除轻击
  (if (`self.IsAttacking`)
    (`PaperZDAnimInstance.StopAllAnimationOverrides` (`self.AnimInstance`))
    (set `self.IsAttacking` false)))

(fn `HeavyAttack`
  (locals (HitActor :type "Actor Object Reference"))
  (bind (_returnvalue_x _returnvalue_y) (`KismetMathLibrary.BreakVector` (* (`self.GetActorForwardVector`) 700.0)))
  (bind _outhits (`self.GetAttackableHits1`))
  (for _array_element _outhits
    (bind _output_get (set `local.HitActor` (`.HitActor` (`GameplayStatics.BreakHitResult` _array_element))))
    (bind _asbp_creature (cast `/Game/Blueprints/Creatures/BP_Creature` _output_get))
    (`self.LaunchCharacter` _asbp_creature (`KismetMathLibrary.MakeVector` _returnvalue_x _returnvalue_y 300.0) false true)
    (`GameplayStatics.ApplyDamage` (`local.HitActor`) (* (`self.AttackValue`) 1.8) null self)))

(fn `UserConstructionScript`
  (`parent.UserConstructionScript`))