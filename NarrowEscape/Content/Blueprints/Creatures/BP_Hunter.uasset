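; BP_Hunter is a sprite-based creature Blueprint that provides a basic attack.
; Attack sphere-sweeps on the AttackChannel along the sprite's forward vector, using configurable offset, length and radius, then applies AttackValue damage to each hit actor.
; Small helper functions separate the range math from the trace.
; The event graph holds only disabled stub events, so nothing here triggers Attack.
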(fn `Attack`
  ; 普通攻击
  (bind _outhits (`self.GetAttackableHits1`))
  (for _array_element _outhits
    (`GameplayStatics.ApplyDamage` (`.HitActor` (`GameplayStatics.BreakHitResult` _array_element)) (`self.AttackValue`) null self)))

(fn `GetAttackableHits`
  (params (Start :type "Vector Structure") (End :type "Vector Structure") (Radius :type "Float (single-precision)"))
  (returns (OutHits :type "Array of HitResult Structure"))
  (locals (_IsSuccess :type Boolean :default false) (_Hits :type "Array of HitResult Structure"))
  ; 球体追踪可攻击Actor
  (bind _outhits (`KismetSystemLibrary.SphereTraceMulti` Start End Radius (`self.AttackChannel`)))
  (return _outhits))

(fn `GetAttackableHits1`
  (returns (OutHits :type "Array of HitResult Structure"))
  (bind (_start _end) (`self.GetSpriteForwardRange` (`self.AttackLength`) (`self.AttackOffset`)))
  (bind _outhits (`self.GetAttackableHits` _start _end (`self.AttackRadius`)))
  (return _outhits))

(fn `GetSpriteForwardRange`
  (params (Length :type "Float (double-precision)") (Offset :type "Float (double-precision)"))
  (returns (Start :type "Vector Structure") (End :type "Vector Structure"))
  (locals (Forward :type "Vector Structure") (_Start :type "Vector Structure") (Forward :type "Vector Structure"))
  (bind _output_get (set `local.Forward` (`SceneComponent.GetForwardVector` (`self.Sprite`))))
  (bind _output_get_2 (set `local._Start` (+ (* (`local.Forward`) Offset) (`self.K2_GetActorLocation`))))
  (return _output_get_2 (+ _output_get_2 (* _output_get Length))))

(fn `UserConstructionScript`
  (`parent.UserConstructionScript`))